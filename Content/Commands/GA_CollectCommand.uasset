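; Gameplay ability that orders the selected units to collect from a targeted resource.
; Triggered by a gameplay event, it runs on authority, unwraps the command data and cancels unless the target implements CollectableResource and reports it can be collected.
; Each commandable unit commits the ability and receives a Command.Resource message through ExecuteCommand.
; CanCommand currently always returns true, leaving its player-ownership check disconnected and unfinished.
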(event Ability|EventActivateAbilityFromEvent
  (params (EventData :type Gameplay%20Event%20Data%20Structure%20%28by%20ref%29))
  (Ability|HasAuthority
    (:True
      (bind _ascommand_event_data_wrapper (Utilities|Casting|CastToCommandEventDataWrapper (.OptionalObject (Utilities|Struct|BreakGameplayEventData EventData)))
        (:then
          (bind _bisvalid (CallFunction|IsValidTarget (.targetactor (Variables|/Script/FirstLine.CommandEventDataWrapper|GetEventData _ascommand_event_data_wrapper))))
          (if _bisvalid
            (for _array_element (.selectedunits (Variables|/Script/FirstLine.CommandEventDataWrapper|GetEventData _ascommand_event_data_wrapper))
              (bind _bvalid (CallFunction|CanCommand _array_element))
              (if _bvalid
                (Ability|CommitAbility)
                (CallFunction|ExecuteCommand _array_element "(TagName=\"Command.Resource\")" (.targetactor (Variables|/Script/FirstLine.CommandEventDataWrapper|GetEventData _ascommand_event_data_wrapper)))
                (else
                  (Ability|EndAbility))))
            (Ability|EndAbility)
            (else
              (Ability|CancelAbility))))
        (:CastFailed
          (Ability|CancelAbility))))
    (:False
      (Ability|EndAbility))))

(fn IsValidTarget
  (params (Target :type Actor%20Object%20Reference))
  (Utilities|IsValid Target
    (:Is%20Valid
      (bind _returnvalue (Class|CollectableResource|CanCollect(Message) Target))
      (return (and (Utilities|DoesObjectImplementInterface Target "/Script/FirstLine.CollectableResource") _returnvalue)))
    (:Is%20Not%20Valid
      (return false))))

(fn CanCommand
  (params (Unit :type Actor%20Object%20Reference))
  (return true))

(fn ExecuteCommand
  (params (Commandable :type Actor%20Object%20Reference) (CommandTag :type Gameplay%20Tag%20Structure) (Target :type Actor%20Object%20Reference))
  (Class|Commandable|ExecuteCommand(Message) Commandable CommandTag (Math|Vector|MakeVector 0.0 0.0 0.0) Target)
  (return))