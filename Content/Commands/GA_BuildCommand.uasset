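; Gameplay ability for an RTS-style build command that places a building and orders the first selected unit to build it.
; On authority, it reads a hard-coded test row from DT_BuildingInfo and uses a BuildingTargetActor with WaitTargetDataUsingActor for user-confirmed placement.
; Confirmation commits, spawns the building and sends Command.Build without ending the ability.
; Unconnected resource-command logic remains, along with its target and ownership check helpers.
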(event Ability|EventActivateAbilityFromEvent
  (params (EventData :type Gameplay%20Event%20Data%20Structure%20%28by%20ref%29))
  (Ability|HasAuthority
    (:True
      (bind _returnvalue (Utilities|GetDataTableRow "/Game/Commands/DT_BuildingInfo.DT_BuildingInfo" "Building.Test")
        (:then
          (bind _returnvalue_2 (Game|SpawnActorfromClass :Class "/Script/FirstLine.BuildingTargetActor" :CollisionHandlingOverride "AlwaysSpawn" :TransformScaleMethod "MultiplyWithRoot" :StartLocation (Utilities|Struct|MakeGameplayAbilityTargetingLocationInfo (Ability|GetAvatarActorfromActorInfo) 0 0 "0.000000,0.000000,0.000000|0.000000,0.000000,-0.000000|1.000000,1.000000,1.000000" "None" "ActorTransform") :ReticleClass 0 :bDebug true :Instigator 0))
          (Class|BuildingTargetActor|SetBuildingClass _returnvalue_2 (.BuildingClass (Utilities|Struct|BreakBuildingData _returnvalue)))
          (bind _data (|WaitTargetDataUsingActor "Find Building Location" "UserConfirmed" _returnvalue_2)
            (:ValidData
              (Ability|CommitAbility)
              (bind _returnvalue_3 (Game|SpawnActorfromClass (.BuildingClass (Utilities|Struct|BreakBuildingData _returnvalue)) (Math|Conversions|ToTransform(Vector) (Class|AbilitySystemBlueprintLibrary|GetTargetDataEndPoint _data)) "Undefined" "MultiplyWithRoot" 0 0))
              (CallFunction|ExecuteCommand (Utilities|Array|Get(acopy) (.selectedunits (Variables|/Script/FirstLine.CommandEventDataWrapper|GetEventData (.AsCommand%20Event%20Data%20Wrapper (Utilities|Casting|CastToCommandEventDataWrapper (.OptionalObject (Utilities|Struct|BreakGameplayEventData EventData))))))) "(TagName=\"Command.Build\")" _returnvalue_3))
            (:Cancelled
              (Development|PrintString "Invalid location")
              (Ability|EndAbility))))))
    (:False
      (Ability|EndAbility))))

(fn IsValidTarget
  (params (Target :type Actor%20Object%20Reference))
  (Utilities|IsValid Target
    (:Is%20Valid
      (bind _returnvalue (Class|CollectableResource|CanCollect(Message) Target))
      (return (and (Utilities|DoesObjectImplementInterface Target "/Script/FirstLine.CollectableResource") _returnvalue)))
    (:Is%20Not%20Valid
      (return false))))

(fn CanCommand
  (params (Unit :type Actor%20Object%20Reference))
  (bind _returnvalue (AI|GetAIController Unit))
  (Utilities|IsValid Unit
    (:Is%20Valid
      (if (Utilities|DoesObjectImplementInterface Unit "/Script/FirstLine.Commandable")
        (Utilities|IsValid _returnvalue
          (:Is%20Valid
            (bind _ascommander_player_state (Utilities|Casting|CastToCommanderPlayerSTate (Variables|/Script/Engine.Controller|GetPlayerState _returnvalue))
              (:then
                (bind _ascommander_player_state_2 (Utilities|Casting|CastToCommanderPlayerSTate (Components|GetOwner (Ability|GetAbilitySystemComponentfromActorInfo)))
                  (:then
                    (return (== (Variables|/Script/Engine.PlayerState|GetPlayerId _ascommander_player_state) (Variables|/Script/Engine.PlayerState|GetPlayerId _ascommander_player_state_2))))
                  (:CastFailed
                    (return false))))
              (:CastFailed
                (return false))))
          (:Is%20Not%20Valid
            (bind _ascommander_player_state_3 (Utilities|Casting|CastToCommanderPlayerSTate (Components|GetOwner Unit))
              (:then
                (bind _ascommander_player_state_4 (Utilities|Casting|CastToCommanderPlayerSTate (Components|GetOwner (Ability|GetAbilitySystemComponentfromActorInfo)))
                  (:then
                    (return (== (Variables|/Script/Engine.PlayerState|GetPlayerId _ascommander_player_state_3) (Variables|/Script/Engine.PlayerState|GetPlayerId _ascommander_player_state_4))))
                  (:CastFailed
                    (return false))))
              (:CastFailed
                (return false)))))
        (else
          _)))
    (:Is%20Not%20Valid
      _))
  (return false))

(fn ExecuteCommand
  (params (Commandable :type Actor%20Object%20Reference) (CommandTag :type Gameplay%20Tag%20Structure) (Target :type Actor%20Object%20Reference))
  (Class|Commandable|ExecuteCommand(Message) Commandable CommandTag (Math|Vector|MakeVector 0.0 0.0 0.0) Target)
  (return))