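; Gameplay Ability that issues a move command to the selected units of a commanding player.
; Triggered by a gameplay event, it reads target location and units from a CommandEventDataWrapper on the authority, cancelling if the payload or navmesh projection fails.
; Each Commandable unit whose owning PlayerState (via AI controller, else the unit) matches the ability owner's PlayerId receives a Command.Move message through the interface.
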(event Ability|EventActivateAbilityFromEvent
  (params (EventData :type Gameplay%20Event%20Data%20Structure%20%28by%20ref%29))
  (Ability|HasAuthority
    (:True
      (bind _ascommand_event_data_wrapper (Utilities|Casting|CastToCommandEventDataWrapper (.OptionalObject (Utilities|Struct|BreakGameplayEventData EventData)))
        (:then
          (bind _bisvalid (CallFunction|IsValidMoveLocation (.targetlocation (Variables|/Script/FirstLine.CommandEventDataWrapper|GetEventData _ascommand_event_data_wrapper))))
          (if _bisvalid
            (for _array_element (.selectedunits (Variables|/Script/FirstLine.CommandEventDataWrapper|GetEventData _ascommand_event_data_wrapper))
              (bind _bvalid (CallFunction|CanCommand _array_element))
              (if _bvalid
                (CallFunction|ExecuteCommand _array_element "(TagName=\"Command.Move\")" (.targetlocation (Variables|/Script/FirstLine.CommandEventDataWrapper|GetEventData _ascommand_event_data_wrapper)))))
            (Ability|EndAbility)
            (else
              (Ability|CancelAbility))))
        (:CastFailed
          (Ability|CancelAbility))))
    (:False
      (Ability|EndAbility))))

(fn IsValidMoveLocation
  (params (Location :type Vector))
  (return (.ReturnValue (AI|Navigation|ProjectPointtoNavigation (Class|NavigationSystemV1|GetNavigationSystem) Location 0 0))))

(fn CanCommand
  (params (Unit :type Actor%20Object%20Reference))
  (bind _returnvalue (AI|GetAIController Unit))
  (Utilities|IsValid Unit
    (:Is%20Valid
      (if (Utilities|DoesObjectImplementInterface Unit "/Script/FirstLine.Commandable")
        (Utilities|IsValid _returnvalue
          (:Is%20Valid
            (bind _ascommander_player_state (Utilities|Casting|CastToCommanderPlayerSTate (Components|GetOwner _returnvalue))
              (:then
                (bind _ascommander_player_state_2 (Utilities|Casting|CastToCommanderPlayerSTate (Components|GetOwner (Ability|GetAbilitySystemComponentfromActorInfo)))
                  (:then
                    (return (== (Variables|/Script/Engine.PlayerState|GetPlayerId _ascommander_player_state) (Variables|/Script/Engine.PlayerState|GetPlayerId _ascommander_player_state_2))))
                  (:CastFailed
                    (return false))))
              (:CastFailed
                (return false))))
          (:Is%20Not%20Valid
            (bind _ascommander_player_state_3 (Utilities|Casting|CastToCommanderPlayerSTate (Components|GetOwner Unit))
              (:then
                (bind _ascommander_player_state_4 (Utilities|Casting|CastToCommanderPlayerSTate (Components|GetOwner (Ability|GetAbilitySystemComponentfromActorInfo)))
                  (:then
                    (return (== (Variables|/Script/Engine.PlayerState|GetPlayerId _ascommander_player_state_3) (Variables|/Script/Engine.PlayerState|GetPlayerId _ascommander_player_state_4))))
                  (:CastFailed
                    (return false))))
              (:CastFailed
                (return false)))))
        (else
          _)))
    (:Is%20Not%20Valid
      _))
  (return false))

(fn ExecuteCommand
  (params (Commandable :type Actor%20Object%20Reference) (CommandTag :type Gameplay%20Tag%20Structure) (Location :type Vector))
  (Class|Commandable|ExecuteCommand(Message) Commandable CommandTag Location)
  (return))