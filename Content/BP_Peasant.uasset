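; BP_Peasant is a selectable peasant actor that always reports it can be selected.
; Its selection events show the R1 component on select and hide it on deselect.
; The construction script creates a dynamic material instance on component R and gives its Color parameter random RGB values, so peasants vary in color.
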(event EventBeginPlay)

(event Collision|EventActorBeginOverlap
  (params (OtherActor :type Actor%20Object%20Reference)))

(event EventTick
  (params (DeltaSeconds :type Float%20%28single-precision%29)))

(event EventOnSelected
  (Development|SetHiddeninGame (Variables|Default|Getr1) false false))

(event EventOnDeselected
  (Development|SetHiddeninGame (Variables|Default|Getr1) true false))

(fn ConstructionScript
  (bind _r (Variables|Default|Getr))
  (bind _returnvalue (Rendering|Material|CreateDynamicMaterialInstance _r 0 (Rendering|Material|GetMaterial _r 0) "None" :!class /Script/Engine.PrimitiveComponent))
  (Rendering|Material|SetVectorParameterValue _returnvalue "Color" (Utilities|Struct|MakeLinearColor (Math|Random|RandomFloat) (Math|Random|RandomFloat) (Math|Random|RandomFloat) 1.0) :!class /Script/Engine.MaterialInstanceDynamic))

(fn CanbeSelected
  (return true))