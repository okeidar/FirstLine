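; BP_Tree is a harvestable wood resource actor that units can gather from through a resource command.
; Query functions report the Wood tag, the Resource command tag, remaining Amount, a fixed collection time and whether anything is left to collect.
; TakeResource subtracts CollectionChunk from Amount, destroys the tree once depleted, and always returns a full chunk of wood, even if less remained.
; All logic lives in these functions; the event graph and construction script are empty.
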(event EventBeginPlay)

(event Collision|EventActorBeginOverlap
  (params (OtherActor :type Actor%20Object%20Reference)))

(event EventTick
  (params (DeltaSeconds :type Float%20%28single-precision%29)))

(fn ConstructionScript)

(fn CanCollect
  (return (> (Variables|Default|GetAmount) 0)))

(fn GetAvailableCommandTags
  (return "(GameplayTags=((TagName=\"Command.Resource\")))"))

(fn GetAvailableResource
  (return (Variables|Default|GetAmount)))

(fn GetCollectionTime
  (return 2.5))

(fn GetResourceTag
  (return "(TagName=\"Resource.Wood\")"))

(fn TakeResource
  (bind _output_get (Variables|Default|SetAmount (- (Variables|Default|GetAmount) (Variables|Default|GetCollectionChunk))))
  (if (> _output_get 0)
    _
    (else
      (Actor|DestroyActor)))
  (return "(TagName=\"Resource.Wood\")" (Variables|Default|GetCollectionChunk)))