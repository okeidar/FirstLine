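; Commander player controller that handles camera movement and drag-box selection.
; It adds the default Enhanced Input mapping context on BeginPlay and forwards move and select actions to camera and selection functions defined outside this graph.
; Selection start, update and end events create, resize and remove a WBP_SelectionBox widget, so the Blueprint supplies only input wiring and the visual box.
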(event Input|EnhancedActionEvents|EnhancedInputActionIA_CameraMove
  (params (ActionValue :type Vector%202D%20Structure) (ElapsedSeconds :type Float%20%28double-precision%29) (TriggeredSeconds :type Float%20%28double-precision%29) (InputAction :type Input%20Action%20Object%20Reference :default "/Game/Input/IA_CameraMove.IA_CameraMove"))
  (Class|CommanderPlayerController|MoveCamerabyInput ActionValue))

(event Input|EnhancedActionEvents|EnhancedInputActionIA_Select
  (params (ActionValue :type Boolean) (ElapsedSeconds :type Float%20%28double-precision%29) (TriggeredSeconds :type Float%20%28double-precision%29) (InputAction :type Input%20Action%20Object%20Reference :default "/Game/Input/IA_Select.IA_Select"))
  (:Started
    (Class|CommanderPlayerController|OnSelectPressed))
  (:Completed
    (Class|CommanderPlayerController|OnSelectReleased)))

(event EventBeginPlay
  (Input|AddMappingContext (PlayerController|LocalPlayerSubsystems|GetEnhancedInputLocalPlayerSubsystem) (Variables|Default|GetDefaultMappingContext) 0 "(bIgnoreAllPressedKeysUntilRelease=True,bForceImmediately=False,bNotifyUserSettings=False)"))

(event EventOnSelectionStarted
  (params (ScreenPosition :type Vector%202D%20Structure%20%28by%20ref%29))
  (bind _returnvalue (UserInterface|CreateWidget "/Game/UI/WBP_SelectionBox.WBP_SelectionBox_C" self ScreenPosition))
  (UserInterface|Viewport|AddtoViewport _returnvalue 0)
  (Variables|Default|SetSelectionBox _returnvalue))

(event EventOnSelectionUpdated
  (params (CurrentScreenPosition :type Vector%202D%20Structure%20%28by%20ref%29))
  (Default|UpdateBox (Variables|Default|GetSelectionBox) CurrentScreenPosition))

(event EventOnSelectionEnded
  (Widget|RemovefromParent (Variables|Default|GetSelectionBox)))

(fn ConstructionScript)